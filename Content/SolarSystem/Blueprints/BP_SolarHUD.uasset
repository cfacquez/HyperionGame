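; HUD for a solar system scene that labels celestial bodies on screen with their name and distance from the camera.
; Each DrawHUD pass finds actors tagged with each BodyNames entry and projects their locations, skipping those behind the camera.
; It draws a short diagonal leader line and text beside each one.
; Distance is rescaled from world units to whole kilometres, switching to astronomical units ("ua") beyond about a tenth of one.
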(event EventBeginPlay)

(event Collision|EventActorBeginOverlap
  (params (OtherActor :type Actor%20Object%20Reference)))

(event EventTick
  (params (DeltaSeconds :type Float%20%28single-precision%29)))

(event EventDrawHUD
  (params (SizeX :type Integer) (SizeY :type Integer))
  (for _array_element (Variables|Default|GetBodyNames)
    (bind _outactors (Actor|GetAllActorswithTag _array_element))
    (for _array_element_2 _outactors
      (if (> (.Z (Math|Vector|BreakVector (Class|HUD|Project (Transformation|GetActorLocation _array_element_2) false))) (Math|Float|MakeLiteralFloat 0.0))
        (Class|HUD|DrawLine (.X (Math|Vector|BreakVector (Class|HUD|Project (Transformation|GetActorLocation _array_element_2) false))) (.Y (Math|Vector|BreakVector (Class|HUD|Project (Transformation|GetActorLocation _array_element_2) false))) (+ (.X (Math|Vector|BreakVector (Class|HUD|Project (Transformation|GetActorLocation _array_element_2) false))) (Math|Float|MakeLiteralFloat 14.0)) (- (.Y (Math|Vector|BreakVector (Class|HUD|Project (Transformation|GetActorLocation _array_element_2) false))) (Math|Float|MakeLiteralFloat 14.0)) (Utilities|Struct|MakeLinearColor 0.6 0.8 1.0 1.0) 1.5)
        (HUD|DrawText (Utilities|String|Append (Utilities|String|Append (Utilities|String|ToString(Name) _array_element) "   ") (Utilities|String|Append (Utilities|String|Replace (Utilities|String|Replace (select (> (/ (Math|Vector|Distance(Vector) (Camera|GetCameraLocation (Game|GetPlayerCameraManager 0)) (Transformation|GetActorLocation _array_element_2)) (Math|Float|MakeLiteralFloat 4e+02)) (Math|Float|MakeLiteralFloat 14959787.07)) (Utilities|String|ToString(Text) (Utilities|Text|ToText(Float) (/ (/ (Math|Vector|Distance(Vector) (Camera|GetCameraLocation (Game|GetPlayerCameraManager 0)) (Transformation|GetActorLocation _array_element_2)) (Math|Float|MakeLiteralFloat 4e+02)) (Math|Float|MakeLiteralFloat 149597870.7)) "HalfToEven" false true 1 324 2 2)) (Utilities|String|ToString(Text) (Utilities|Text|ToText(String) (Class|KismetMathLibrary|FTrunc64 (/ (Math|Vector|Distance(Vector) (Camera|GetCameraLocation (Game|GetPlayerCameraManager 0)) (Transformation|GetActorLocation _array_element_2)) (Math|Float|MakeLiteralFloat 4e+02)))))) " " " ") " " " ") (select (> (/ (Math|Vector|Distance(Vector) (Camera|GetCameraLocation (Game|GetPlayerCameraManager 0)) (Transformation|GetActorLocation _array_element_2)) (Math|Float|MakeLiteralFloat 4e+02)) (Math|Float|MakeLiteralFloat 14959787.07)) (Utilities|String|MakeLiteralString " ua") (Utilities|String|MakeLiteralString " km")))) (Utilities|Struct|MakeLinearColor 0.85 0.92 1.0 1.0) (+ (.X (Math|Vector|BreakVector (Class|HUD|Project (Transformation|GetActorLocation _array_element_2) false))) (Math|Float|MakeLiteralFloat 16.0)) (- (.Y (Math|Vector|BreakVector (Class|HUD|Project (Transformation|GetActorLocation _array_element_2) false))) (Math|Float|MakeLiteralFloat 3e+01)) 0 1.3 false)))))

(fn ConstructionScript)